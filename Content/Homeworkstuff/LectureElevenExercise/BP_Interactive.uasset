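; BP_Interactive is an interactable object with a Use function, which also contains the E key handler that triggers interaction.
; Pressing E line traces 300 units forward from player camera 0 against WorldDynamic objects.
; A hit actor that casts to BP_Interactive gets its Use called, which here only prints a placeholder message.
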(event `Key|E`
  (params (Key :type "Key Structure"))
  (bind _returnvalue (`GameplayStatics.GetPlayerCameraManager` 0))
  (bind _returnvalue_2 (`self.K2_GetActorLocation` _returnvalue))
  (:`Pressed`
    (bind (_outhit _returnvalue_3) (`KismetSystemLibrary.LineTraceSingleForObjects` _returnvalue_2 (+ _returnvalue_2 (* (`self.GetActorForwardVector` _returnvalue) (300.0 300.0 300.0))) (`|MakeArray` "ObjectTypeQuery2" :!type "EObjectTypeQuery Enum")))
    (if _returnvalue_3
      (bind _asbp_interactive (cast `/Game/Homeworkstuff/LectureElevenExercise/BP_Interactive` (`.HitActor` (`GameplayStatics.BreakHitResult` _outhit))))
      (`self.Use` _asbp_interactive))))

(fn `Use`
  (`KismetSystemLibrary.PrintString` "OBJECT IN USE"))

(fn `UserConstructionScript`)